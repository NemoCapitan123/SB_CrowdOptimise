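; Spawner actor that creates a crowd of unoptimised AI bots (BPAIBotDCMNoOptimise) when ThirdPersonCharacterMain steps on InterractPlate.
; Two sequential counter loops spawn 50 bots each in rows along Y, the second from a hard-coded start position.
; CountBots resets only between loops, so later overlaps skip the first row and spawn the second again.
; An unconnected block for 100 more bots never runs.
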(event `self.InterractPlate.OnComponentBeginOverlap`
  (params (OverlappedComponent :type "PrimitiveComponent Object Reference") (OtherActor :type "Actor Object Reference") (OtherComp :type "PrimitiveComponent Object Reference") (OtherBodyIndex :type Integer) (bFromSweep :type Boolean) (SweepResult :type "HitResult Structure (by ref)"))
  (bind (_spawn_transform_x _spawn_transform_y _spawn_transform_z) (`KismetMathLibrary.BreakVector` (`self.Spawn Transform`)))
  (bind (_spawn_transform_x_2 _spawn_transform_y_2 _spawn_transform_z_2) (`KismetMathLibrary.BreakVector` (`self.Spawn Transform`)))
  (bind _returnvalue (`KismetMathLibrary.MakeVector` _spawn_transform_x (+ _spawn_transform_y 100.0) _spawn_transform_z))
  (bind _returnvalue_2 (`KismetMathLibrary.MakeVector` _spawn_transform_x_2 (+ _spawn_transform_y_2 100.0) _spawn_transform_z_2))
  (bind _returnvalue_3 (not (>= (`self.CountBots`) 50)))
  (cast `/Game/AI/ThirdPersonCharacterMain` OtherActor)
  (while _returnvalue_3
    (set `self.Spawn Transform` _returnvalue)
    (`|SpawnActorFromClass` "/Game/AI/BPAIBotDCMNoOptimise.BPAIBotDCMNoOptimise_C" (`KismetMathLibrary.MakeTransform` _returnvalue) "Undefined" "OverrideRootScale" null null)
    (`/Engine/EditorBlueprintResources/StandardMacros.IncrementInt` (`self.CountBots`)))
  (set `self.CountBots` 0)
  (set `self.Spawn Transform` (-20.0 -3000.0 142.0))
  (while _returnvalue_3
    (set `self.Spawn Transform` _returnvalue_2)
    (`|SpawnActorFromClass` "/Game/AI/BPAIBotDCMNoOptimise.BPAIBotDCMNoOptimise_C" (`KismetMathLibrary.MakeTransform` _returnvalue_2) "Undefined" "OverrideRootScale" null null)
    (`/Engine/EditorBlueprintResources/StandardMacros.IncrementInt` (`self.CountBots`))))

(event `self.ReceiveBeginPlay`)

(fn `UserConstructionScript`)